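; BP_Magnet is a magnet power-up pickup for the runner game.
; When the runner character overlaps it, it plays a sound, hides itself and, if no magnet is active, sets IsMagnetActive on the character for five seconds.
; The actor is hidden rather than destroyed, and its own delay clears the flag.
; It also destroys any wall, blocker or coin that overlaps it.
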(event `self.ReceiveActorBeginOverlap`
  (params (OtherActor :type "Actor Object Reference"))
  (`|ExecutionSequence`
    (:`then_0`
      (bind _asbp_runner_character (cast `/Game/Runner/Blueprints/BP_RunnerCharacter` OtherActor))
      (cast `/Game/Runner/Blueprints/BP_RunnerGameMode` (`GameplayStatics.GetGameMode`))
      (`GameplayStatics.PlaySound2D` "/Engine/VREditor/Sounds/UI/Object_Snaps_To_Another_Actor.Object_Snaps_To_Another_Actor" 1.0 1.0 0.0 null null)
      (`self.SetActorHiddenInGame` true)
      (if (not (`/Game/Runner/Blueprints/BP_RunnerCharacter.isMagnetActive` _asbp_runner_character))
        (bind _output_get (set `/Game/Runner/Blueprints/BP_RunnerCharacter.isMagnetActive` true _asbp_runner_character))
        (`KismetSystemLibrary.PrintString` (`KismetStringLibrary.Conv_BoolToString` _output_get))
        (`KismetSystemLibrary.Delay` 5.0)
        (bind _asbp_runner_character_2 (cast `/Game/Runner/Blueprints/BP_RunnerCharacter` (`GameplayStatics.GetPlayerCharacter` 0)))
        (bind _output_get_2 (set `/Game/Runner/Blueprints/BP_RunnerCharacter.isMagnetActive` false _asbp_runner_character_2))
        (`KismetSystemLibrary.PrintString` (`KismetStringLibrary.Conv_BoolToString` _output_get_2))))
    (:`then_1`
      (bind _asbp_obsacles_wall (cast `/Game/Runner/Blueprints/Obsacles/BP_Obsacles_Wall` OtherActor))
      (`self.K2_DestroyActor` _asbp_obsacles_wall))
    (:`then_2`
      (bind _asbp_coin (cast `/Game/Runner/Blueprints/BP_Coin` OtherActor))
      (`self.K2_DestroyActor` _asbp_coin))
    (:`then_3`
      (bind _asbp_obsacles_blocker (cast `/Game/Runner/Blueprints/Obsacles/BP_Obsacles_Blocker` OtherActor))
      (`self.K2_DestroyActor` _asbp_obsacles_blocker))))

(fn `UserConstructionScript`)