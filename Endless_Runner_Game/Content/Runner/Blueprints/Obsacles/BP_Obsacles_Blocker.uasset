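; Runner obstacle blocker that kills the player character on overlap unless that character is sliding.
; On a fatal hit it calls the character's Death, then pauses the game after a short delay.
; The construction script gives each of its three static meshes a dynamic instance of the Random_Color material with its own random color.
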(event `self.ReceiveActorBeginOverlap`
  (params (OtherActor :type "Actor Object Reference"))
  (bind _asbp_runner_character (cast `/Game/Runner/Blueprints/BP_RunnerCharacter` OtherActor))
  (if (not (`/Game/Runner/Blueprints/BP_RunnerCharacter.isSliding` _asbp_runner_character))
    (`/Game/Runner/Blueprints/BP_RunnerCharacter.Death` _asbp_runner_character)
    (`KismetSystemLibrary.Delay` 1.0)
    (`GameplayStatics.SetGamePaused` true)))

(fn `UserConstructionScript`
  (bind _returnvalue (`KismetMathLibrary.RandomFloat`))
  (bind _returnvalue_2 (`KismetMathLibrary.RandomFloat`))
  (bind _returnvalue_3 (`KismetMathLibrary.RandomFloat`))
  (bind _returnvalue_4 (`PrimitiveComponent.CreateDynamicMaterialInstance` (`self.StaticMesh`) 0 "/Game/Runner/Materials/Random_Color.Random_Color" "None"))
  (`MaterialInstanceDynamic.SetVectorParameterValue` _returnvalue_4 "Color" (make `LinearColor` _returnvalue _returnvalue_3 _returnvalue_2 1.0))
  (bind _returnvalue_5 (`PrimitiveComponent.CreateDynamicMaterialInstance` (`self.StaticMesh1`) 0 "/Game/Runner/Materials/Random_Color.Random_Color" "None"))
  (`MaterialInstanceDynamic.SetVectorParameterValue` _returnvalue_5 "Color" (make `LinearColor` _returnvalue _returnvalue_3 _returnvalue_2 1.0))
  (bind _returnvalue_6 (`PrimitiveComponent.CreateDynamicMaterialInstance` (`self.StaticMesh2`) 0 "/Game/Runner/Materials/Random_Color.Random_Color" "None"))
  (`MaterialInstanceDynamic.SetVectorParameterValue` _returnvalue_6 "Color" (make `LinearColor` _returnvalue _returnvalue_3 _returnvalue_2 1.0))
  (`parent.UserConstructionScript`))