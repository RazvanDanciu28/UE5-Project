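; Floor tile for an endless runner that exposes its Arrow transform as the attach point for chaining tiles.
; Construction builds two rows of spawn points across the lane positions, then shuffles them to place one or two child-actor obstacles, randomly choosing between two spawn nodes.
; When the runner character overlaps the Box trigger, the tile tells the game mode to extend the floor and adds a point to the score.
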(event `self.ReceiveBeginPlay`)

(event `self.Box.OnComponentBeginOverlap`
  (params (OverlappedComponent :type "PrimitiveComponent Object Reference") (OtherActor :type "Actor Object Reference") (OtherComp :type "PrimitiveComponent Object Reference") (OtherBodyIndex :type Integer) (bFromSweep :type Boolean) (SweepResult :type "HitResult Structure (by ref)"))
  ;[1 1 1] extend field
  (cast `/Game/Runner/Blueprints/BP_RunnerCharacter` OtherActor)
  (bind _asbp_runner_game_mode (cast `/Game/Runner/Blueprints/BP_RunnerGameMode` (`GameplayStatics.GetGameMode`)))
  (`/Game/Runner/Blueprints/BP_RunnerGameMode.Extend Floor` _asbp_runner_game_mode)
  ;[1 1 1] Set Score
  (bind _asbp_runner_game_mode_2 (cast `/Game/Runner/Blueprints/BP_RunnerGameMode` (`GameplayStatics.GetGameMode`)))
  (set `/Game/Runner/Blueprints/BP_RunnerGameMode.currentPoints` (+ (`/Game/Runner/Blueprints/BP_RunnerGameMode.currentPoints` _asbp_runner_game_mode_2) 1) _asbp_runner_game_mode_2))

(fn `Get Attach Point`
  (returns (ReturnValue :type "Transform Structure"))
  (return (`SceneComponent.K2_GetComponentToWorld` (`self.Arrow`))))

(fn `Setup Spawn Points`
  (for _array_element (`self.Lane Position`)
    (for _index (range 2)
      (bind _returnvalue (`AddComponent|NODE_AddArrowComponent-0` :`RelativeTransform` (`KismetMathLibrary.MakeTransform` (`KismetMathLibrary.MakeVector` (* _index 650.0) _array_element))))
      (`KismetArrayLibrary.Array_Add` (`self.Spaw Points`) (`SceneComponent.K2_GetComponentToWorld` _returnvalue)))))

(fn `Spaw Obsacles`
  (locals (`Random Spaw Points` :type "Array of Transform Structure"))
  (bind _output_get (set `local.Random Spaw Points` (`self.Spaw Points`)))
  (`KismetArrayLibrary.Array_Shuffle` _output_get)
  (for _index (range (+ (`KismetMathLibrary.RandomIntegerInRange` 0 1) 1))
    (switch `int` (`KismetMathLibrary.RandomIntegerInRange` 0 1)
      (:`0`
        (bind _returnvalue (`KismetMathLibrary.MakeRelativeTransform` (`|GetArrayItem` (`local.Random Spaw Points`) _index) (`self.GetTransform`)))
        (`AddComponent|NODE_AddChildActorComponent-0` :`RelativeTransform` _returnvalue))
      (:`1`
        (`AddComponent|NODE_AddChildActorComponent-1` :`RelativeTransform` _returnvalue)))))

(fn `UserConstructionScript`
  (`self.Setup Spawn Points`)
  (`self.Spaw Obsacles`))